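; BP_EnemyActor is a destructible enemy block with a random sprite variant and a matching score bonus.
; SetEnemyEvent rolls cascading chances, retrying until one of four tiers hits, then sets the flipbook and Bonus from that tier; ZIndex is unused.
; On destruction it spawns an explosion, then has BP_GameMode add the Bonus and check for a win.
; DropBombEvent is an empty stub, with its bomb spawn node left unconnected.
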(event `Set Enemy Event`
  (params (`Z Index` :type Integer))
  (bind _spawnchance (`self.SpawnChance`))
  ;[1 1 1] set bonus for each bloc
  (if (< (`KismetMathLibrary.RandomInteger` 100) 50) :!label _label
    (set `self.SpawnChance` 0)
    (elif (< (`KismetMathLibrary.RandomInteger` 100) 25)
      (set `self.SpawnChance` 1)
      (elif (< (`KismetMathLibrary.RandomInteger` 100) 15)
        (set `self.SpawnChance` 2)
        (elif (< (`KismetMathLibrary.RandomInteger` 100) 10)
          (set `self.SpawnChance` 3)
          (else
            (goto _label))))))
  (`PaperFlipbookComponent.SetFlipbook` (`self.EnemyFlipbook`) (select `int` _spawnchance :`0` "/Game/Assets/FlipBooks/b1.b1" :`1` "/Game/Assets/FlipBooks/b3.b3" :`2` "/Game/Assets/FlipBooks/b4.b4" :`3` "/Game/Assets/FlipBooks/b5.b5" :!type "PaperFlipbook Object Reference"))
  (set `self.Bonus` (select `int` _spawnchance :`0` 10 :`1` 20 :`2` 40 :`3` 50 :`4` 80)))

(event `self.ReceiveDestroyed`
  ;[1 1 1] add point for a destroyed bloc and check win
  (`|SpawnActorFromClass` "/Game/Blueprints/BP_ExplosionActor.BP_ExplosionActor_C" (`KismetMathLibrary.MakeTransform` (`self.K2_GetActorLocation`)) "AdjustIfPossibleButDontSpawnIfColliding" "OverrideRootScale" null null)
  (bind _asbp_game_mode (cast `/Game/Blueprints/BP_GameMode` (`GameplayStatics.GetGameMode`)))
  (`/Game/Blueprints/BP_GameMode.Update Score Event` _asbp_game_mode (`self.Bonus`))
  (`/Game/Blueprints/BP_GameMode.Check Winning Event` _asbp_game_mode))

(event `Drop Bomb Event`)

(fn `UserConstructionScript`)