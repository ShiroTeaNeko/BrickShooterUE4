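; Game mode for a Space Invaders-style shooter, running player spawning, score, lives, HUD, win/lose screen and restart.
; Enemy grids attach to group actors that shift sideways through a gate, with direction reversal left unwired.
; A Delay-throttled Tick counter steps groups downward and spawns another grid every fourth step.
; A looping timer makes random enemies drop bombs, and win checks speed up the wave while enemies remain.
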(event `Start New Game Event`
  ;[1 1 1] NG
  (`|ExecutionSequence`
    (:`then_0`
      (`self.Spawn Player Event`))
    (:`then_1`
      (`self.Spawn Blocs Events`))
    (:`then_2`
      (`self.MoveWaveEvent`)
      (bind _returnvalue (`KismetSystemLibrary.K2_SetTimer` self "Spawn Random Bombs" 2.0 true))
      (set `self.SpawnBombTimerHandle` _returnvalue))
    (:`then_3`
      (bind _returnvalue_2 (`|CreateWidget` "/Game/Blueprints/Widgets/WG_GameHUD.WG_GameHUD_C"))
      (bind _output_get (set `self.GameHUD_Ref` _returnvalue_2))
      (`UserWidget.AddToViewport` _output_get 0)
      (`/Game/Blueprints/Widgets/WG_GameHUD.Update Score Text` _output_get 0))))

(event `MoveWaveEvent`
  ;[1 1 1] move bloc
  (`/Engine/EditorBlueprintResources/StandardMacros.Gate` true :!via `Open` :!label _label
    (:`Exit`
      (for _array_element (`self.arrayActorRef`)
        (`self.K2_AddActorWorldOffset` _array_element (`KismetMathLibrary.MakeVector` (* (`self.WaveSpeed`) (`GameplayStatics.GetWorldDeltaSeconds`) (`self.MovementDirection`))) false false)))))

(event `StopWaveEvent`
  ;[1 1 1] move bloc
  (goto _label :!via `Close`))

(event `Spawn Player Event`
  ;[1 1 1] spawn player
  (bind _returnvalue (`|SpawnActorFromClass` "/Game/Blueprints/BP_PlayerShipPawn.BP_PlayerShipPawn_C" (`KismetMathLibrary.MakeTransform` (0.0 0.0 -480.0) (struct) (0.2 0.2 0.2)) "AdjustIfPossibleButDontSpawnIfColliding" "OverrideRootScale" null null))
  (set `self.PlayerActor_Ref` _returnvalue))

(event `InverseDirectionEvent`)

(event `self.ReceiveTick`
  (params (DeltaSeconds :type "Float (single-precision)"))
  ;[1 1 1] Chrono
  (`KismetSystemLibrary.Delay` (`self.BlocSpeed`))
  (set `self.TimeSec` (+ (`self.TimeSec`) 1))
  (if (> (`self.TimeSec`) 1)
    (set `self.chiffre` (+ (`self.chiffre`) 1))
    (`self.MoveWaveDownEvent`)
    (set `self.TimeSec` 0)
    (if (>= (`self.chiffre`) 4)
      (`self.Spawn Blocs Events`)
      (set `self.chiffre` 0))))

(event `MoveWaveDownEvent`
  ;[1 1 1] move down blocs
  (for _array_element (`self.arrayActorRef`)
    (bind (_returnvalue_x _returnvalue_y _returnvalue_z) (`KismetMathLibrary.BreakVector` (`self.K2_GetActorLocation` _array_element)))
    (`self.K2_SetActorLocation` _array_element (`KismetMathLibrary.MakeVector` _returnvalue_x _returnvalue_y (- _returnvalue_z 20.0)) false false)))

(event `Spawn Blocs Events`
  ;[1 1 1] spawn blocs
  (bind _returnvalue (`|SpawnActorFromClass` "/Game/Blueprints/BP_EnemiesGroupActor.BP_EnemiesGroupActor_C" (`KismetMathLibrary.MakeTransform` (`self.Wave Start Location`) (struct) (1.0 1.0 1.0)) "AdjustIfPossibleButAlwaysSpawn" "OverrideRootScale" null null))
  (bind _outactors (`GameplayStatics.GetAllActorsOfClass` "/Game/Blueprints/BP_EnemiesGroupActor.BP_EnemiesGroupActor_C"))
  (set `self.arrayActorRef` _outactors)
  (set `self.GroupActor_Ref` _returnvalue)
  (for _index (range (* (`self.Horizontal Enemies Count`) (`self.Vertical Enemies Count`)))
    (`self.Spawn New Bloc` (mod _index (`self.Horizontal Enemies Count`)) (/ _index (`self.Horizontal Enemies Count`)))))

(event `Update Score Event`
  (params (Bonus :type Integer))
  ;[1 1 1] Update of Score
  (bind _output_get (set `self.Score` (+ Bonus (`self.Score`))))
  (`/Game/Blueprints/Widgets/WG_GameHUD.Update Score Text` (`self.GameHUD_Ref`) _output_get))

(event `Speed Up Wave Movement Event`
  (set `self.WaveSpeed` (+ (`self.WaveSpeed`) 5.0)))

(event `Check Winning Event`
  ;[1 1 1] Check for a win
  (bind _outactors (`GameplayStatics.GetAllActorsOfClass` "/Game/Blueprints/BP_EnemyActor.BP_EnemyActor_C"))
  (if (<= (`KismetArrayLibrary.Array_Length` _outactors) 1)
    (`self.End Game Event` true)
    (else
      (`self.Speed Up Wave Movement Event`))))

(event `Lives Update Event`
  (`/Engine/EditorBlueprintResources/StandardMacros.CompareInt` (`self.Lives`) 1
    (:`>`
      (`KismetSystemLibrary.K2_PauseTimerHandle` (`self.SpawnBombTimerHandle`))
      (`self.StopWaveEvent`)
      (set `self.Lives` (- (`self.Lives`) 1))
      (`/Game/Blueprints/Widgets/WG_GameHUD.Update Lives Texture` (`self.GameHUD_Ref`) (`self.Lives`))
      (`KismetSystemLibrary.Delay` 0.5)
      (`self.Spawn Player Event`)
      (`KismetSystemLibrary.K2_UnPauseTimerHandle` (`self.SpawnBombTimerHandle`))
      (`self.MoveWaveEvent`))
    (:`==`
      (`self.StopWaveEvent`)
      (`self.Game Over Event`))))

(event `End Game Event`
  (params (`Won?` :type Boolean))
  (bind _returnvalue (`GameplayStatics.GetPlayerController` 0))
  ;[1 1 1] show End screen
  (bind _returnvalue_2 (`|CreateWidget` "/Game/Blueprints/Widgets/WG_GameEnd.WG_GameEnd_C"))
  (bind _output_get (set `self.GameEndWidget_Ref` _returnvalue_2))
  (`/Game/Blueprints/Widgets/WG_GameEnd.Set Game End Message` _output_get `Won?`)
  (`UserWidget.AddToViewport` _output_get 0)
  (set `PlayerController.bShowMouseCursor` true _returnvalue)
  (`/Engine/EditorBlueprintResources/StandardMacros.IsValid` (`self.PlayerActor_Ref`)
    (:`Is Valid`
      (`self.DisableInput` (`self.PlayerActor_Ref`) _returnvalue))))

(event `Game Over Event`
  (bind _playeractor_ref (`self.PlayerActor_Ref`))
  ;[1 1 1] if GameOver
  (set `self.Lives` 0)
  (`/Game/Blueprints/Widgets/WG_GameHUD.Update Lives Texture` (`self.GameHUD_Ref`) 0)
  (`self.StopWaveEvent`)
  (`|ExecutionSequence`
    (:`then_0`
      (`/Engine/EditorBlueprintResources/StandardMacros.IsValid` _playeractor_ref
        (:`Is Valid`
          (`self.K2_DestroyActor` _playeractor_ref))))
    (:`then_1`
      (`KismetSystemLibrary.Delay` 0.5)
      (`self.End Game Event` false))))

(event `Restart Game Event`
  (`Widget.RemoveFromParent` (`self.GameHUD_Ref`))
  (`Widget.RemoveFromParent` (`self.GameEndWidget_Ref`))
  (`GameplayStatics.OpenLevel` "MainGame_Map"))

(fn `Spawn New Bloc`
  (params (`X Index` :type Integer) (`Y Index` :type Integer))
  ;[1 1 1] Spawn Group of bloc
  (bind _returnvalue (`|SpawnActorFromClass` "/Game/Blueprints/BP_EnemyActor.BP_EnemyActor_C" (`KismetMathLibrary.MakeTransform` (+ (`self.Wave Start Location`) (* (`KismetMathLibrary.MakeVector` (`KismetMathLibrary.Conv_IntToDouble` `X Index`) 0.0 (`KismetMathLibrary.Conv_IntToDouble` `Y Index`)) (`self.Spacing`))) (struct) (2.0 1.0 2.0)) "AdjustIfPossibleButDontSpawnIfColliding" "OverrideRootScale" null null))
  (`/Game/Blueprints/BP_EnemyActor.Set Enemy Event` _returnvalue `Y Index`)
  (for _array_element (`self.arrayActorRef`)
    (`self.K2_AttachRootComponentToActor` _returnvalue _array_element "None" "KeepWorldPosition" true)))

(fn `Spawn Random Bombs`
  (locals (EnemiesTempArray :type "Array of /Game/Blueprints/BP_EnemyActor Object Reference"))
  (bind _enemiestemparray (`local.EnemiesTempArray`))
  (bind _output (`|GetArrayItem` _enemiestemparray))
  (bind _outactors (`GameplayStatics.GetAllActorsOfClass` "/Game/Blueprints/BP_EnemyActor.BP_EnemyActor_C"))
  (set `local.EnemiesTempArray` _outactors)
  (for _ (range (+ (`KismetMathLibrary.RandomIntegerInRange` 1 3) 1))
    (`KismetArrayLibrary.Array_Shuffle` _enemiestemparray)
    (`/Engine/EditorBlueprintResources/StandardMacros.IsValid` _output
      (:`Is Valid`
        (`/Game/Blueprints/BP_EnemyActor.Drop Bomb Event` _output)
        (`KismetArrayLibrary.Array_RemoveItem` (`local.EnemiesTempArray`) _output)))))

(fn `UserConstructionScript`)