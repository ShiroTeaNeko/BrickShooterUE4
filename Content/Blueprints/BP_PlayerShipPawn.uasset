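; Player ship pawn for a shooter, sliding along the X axis within fixed bounds and firing lasers.
; Shoot spawns a laser through a DoOnce that resets shortly after release, so each press fires at most one shot.
; When destroyed, it spawns an explosion and tells BP_GameMode to update lives.
; Overlapping a BP_EnemyActor triggers the game mode's game over event directly.
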(event `self.ReceiveDestroyed`
  (`|SpawnActorFromClass` "/Game/Blueprints/BP_ExplosionActor.BP_ExplosionActor_C" (`KismetMathLibrary.MakeTransform` (`self.K2_GetActorLocation`)) "AdjustIfPossibleButDontSpawnIfColliding" "OverrideRootScale" null null)
  (bind _asbp_game_mode (cast `/Game/Blueprints/BP_GameMode` (`GameplayStatics.GetGameMode`)))
  (`/Game/Blueprints/BP_GameMode.Lives Update Event` _asbp_game_mode))

(event `InputAxis|MoveRight`
  (params (AxisValue :type "Float (single-precision)"))
  (bind (_returnvalue_x _returnvalue_y _returnvalue_z) (`KismetMathLibrary.BreakVector` (`self.K2_GetActorLocation`)))
  ;[1 1 1] move in line
  (`self.K2_AddActorWorldOffset` (* (1.0 0.0 0.0) (* AxisValue (`self.Speed`) (`GameplayStatics.GetWorldDeltaSeconds`))))
  (`self.K2_SetActorLocation` (`KismetMathLibrary.MakeVector` (`KismetMathLibrary.FClamp` _returnvalue_x -850.0 850.0) _returnvalue_y _returnvalue_z)))

(event `InputAction|Shoot`
  (params (Key :type "Key Structure"))
  ;[1 1 1] fire a missile
  (:`Pressed`
    (`/Engine/EditorBlueprintResources/StandardMacros.DoOnce` false :!label _label
      (:`Completed`
        (`|SpawnActorFromClass` "/Game/Blueprints/BP_LaserActor.BP_LaserActor_C" (`KismetMathLibrary.MakeTransform` (`self.K2_GetActorLocation`) (struct) (1.0 1.0 1.0)) "AlwaysSpawn" "OverrideRootScale" null null))))
  (:`Released`
    (`KismetSystemLibrary.Delay` 0.3)
    (goto _label :!via `Reset`)))

(event `self.ReceiveActorBeginOverlap`
  (params (OtherActor :type "Actor Object Reference"))
  ;[1 1 1] if player is overlapped by bloc then GameOver
  (cast `/Game/Blueprints/BP_EnemyActor` OtherActor)
  (bind _asbp_game_mode (cast `/Game/Blueprints/BP_GameMode` (`GameplayStatics.GetGameMode`)))
  (`/Game/Blueprints/BP_GameMode.Game Over Event` _asbp_game_mode))

(fn `UserConstructionScript`)